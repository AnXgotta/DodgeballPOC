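; BP_TestBall is a dodgeball test Blueprint that traces the trajectory of its Sphere component with persistent debug lines.
; BeginPlay stores the sphere's world location, then Tick draws a segment and updates that stored position whenever the sphere has moved beyond a small distance threshold.
; The Hit event and construction script are empty, and a gravity-enabling branch is left unconnected.
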(event `self.ReceiveHit`
  (params (MyComp :type "PrimitiveComponent Object Reference") (Other :type "Actor Object Reference") (OtherComp :type "PrimitiveComponent Object Reference") (bSelfMoved :type Boolean) (HitLocation :type "Vector Structure") (HitNormal :type "Vector Structure") (NormalImpulse :type "Vector Structure") (Hit :type "HitResult Structure (by ref)")))

(event `self.ReceiveBeginPlay`
  (`|ExecutionSequence`
    (:`then_0`
      ;[1 0.3422 0.2656] Debug Trajectory
      (set `self.PreviousPosition` (`SceneComponent.K2_GetComponentLocation` (`self.Sphere`))))))

(event `self.ReceiveTick`
  (params (DeltaSeconds :type "Float (single-precision)"))
  (bind _returnvalue (`SceneComponent.K2_GetComponentLocation` (`self.Sphere`)))
  (`|ExecutionSequence`
    (:`then_0`
      ;[1 0.3422 0.2656] Debug Trajectory
      (if (> (`KismetMathLibrary.VSize` (- (`self.PreviousPosition`) _returnvalue)) 10.0)
        (`|ExecutionSequence`
          (:`then_0`
            (`KismetSystemLibrary.DrawDebugLine` (stale _output_get) _returnvalue (struct :`G` 0.014613 :`B` 1.0 :`A` 1.0) 9999.0 2.0))
          (:`then_1`
            (bind _output_get (set `self.PreviousPosition` _returnvalue))))))))

(fn `UserConstructionScript`)